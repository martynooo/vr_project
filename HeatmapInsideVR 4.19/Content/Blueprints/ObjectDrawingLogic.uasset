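; Drawable object logic that records brush splats into a render target and displays them as a heat map on the object.
; The construction script creates dynamic instances of the splat brush and heat map display materials.
; DrawToRenderTargetUsingUV sets the brush's UV position, strength and size, then draws it into the render target.
; ShowHeatmaps binds that render target to the display material and flip-flops Base between it and the initial material.
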(event Custom|DrawToRenderTargetUsingUV
  (params (Location :type Vector%202D%20Structure) (Strength :type Float%20%28single-precision%29) (Size :type Float%20%28single-precision%29))
  (bind _mid_heatsplat (Variables|Default|GetMID_Heatsplat))
  (Rendering|Material|SetScalarParameterValue _mid_heatsplat "Strength" Strength :!class /Script/Engine.MaterialInstanceDynamic)
  (Rendering|Material|SetScalarParameterValue _mid_heatsplat "Size" Size :!class /Script/Engine.MaterialInstanceDynamic)
  (Rendering|Material|SetVectorParameterValue _mid_heatsplat "Position" (Math|Conversions|ToLinearColor(Vector) (Math|Conversions|ToVector(Vector2D) Location)) :!class /Script/Engine.MaterialInstanceDynamic)
  (Rendering|DrawMaterialtoRenderTarget (Variables|Default|GetRenderTarget) _mid_heatsplat))

(event Custom|ShowHeatmaps
  (bind _heatsplatcolor (Variables|Default|GetHeatSplatColor))
  (bind _base (Variables|Default|GetBase))
  (Rendering|Material|SetTextureParameterValue _heatsplatcolor "RenderTarget" (Variables|Default|GetRenderTarget))
  (Utilities|FlowControl|FlipFlop
    (:A
      (Rendering|Material|SetMaterial _base 0 _heatsplatcolor))
    (:B
      (Rendering|Material|SetMaterial _base 0 (Variables|Default|GetInitMaterial)))))

(fn ConstructionScript
  (bind _returnvalue (Rendering|Material|CreateDynamicMaterialInstance "/Game/Materials/HeatSplatColor.HeatSplatColor" :!class /Script/Engine.KismetMaterialLibrary))
  (Variables|Default|SetHeatSplatColor _returnvalue)
  (bind _returnvalue_2 (Rendering|Material|CreateDynamicMaterialInstance "/Game/Materials/HeatSplat.HeatSplat" :!class /Script/Engine.KismetMaterialLibrary))
  (Variables|Default|SetMID_Heatsplat _returnvalue_2))